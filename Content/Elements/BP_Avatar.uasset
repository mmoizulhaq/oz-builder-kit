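; Bitmoji dancer avatar that loads its glTF model at runtime on BeginPlay, named by Filename or the first BP_ModelTracker.
; HighResolution selects LOD0 or LOD3; meshes merge onto a forced BitmojiSkeleton, and capsule and mesh offset follow the bounds.
; High resolution also loads facial morph-curve animations, played randomly in the Face slot by a self-rescheduling timer.
; The timer's duration is drawn by a separate random pick from the animation's.
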(event Custom|PlayFacialAnimation
  ;[1 1 1] Randomly play a facial animation
  (bind (_animation _duration) (CallFunction|GetRandomFacialAnimation))
  (Class|AnimInstance|PlaySlotAnimationasDynamicMontage (Components|SkeletalMesh|GetAnimInstance (Variables|Character|GetMesh)) _animation "Face" 0.25 0.25 1.0 1 -1.0 0.0)
  (Utilities|Time|SetTimerbyEvent (delegate Custom|PlayFacialAnimation) _duration))

(event EventBeginPlay
  (if (Utilities|Enum|Equal(Enum) (Variables|Default|GetFilename) "")
    (bind _outactors (Actor|GetAllActorsOfClass "/OZFusion/Elements/BP_ModelTracker.BP_ModelTracker_C"))
    (bind _array_element (Utilities|Array|ForEachLoopwithBreak _outactors :!label _label)
      (:LoopBody
        (bind _filename (Default|ReturnFilename _array_element))
        (Variables|Default|SetFullPath (Utilities|String|Append "Models/" _filename (Utilities|String|SelectString "_lod0.glb" "_lod3.glb" (Variables|Default|GetHighResolution))))
        (goto _label Break))
      (:Completed
        _))
    (else
      (Variables|Default|SetFullPath (Utilities|String|Append "Models/" (Variables|Default|GetFilename) (Utilities|String|SelectString "_lod0.glb" "_lod3.glb" (Variables|Default|GetHighResolution))))))
  ;[1 1 1] load asset
  (bind _returnvalue (Class|GlTFRuntimeFunctionLibrary|GlTFLoadAssetfromFilename (Variables|Default|GetFullPath) true (Utilities|Struct|MakeglTFRuntimeConfig "Default" "(XPlane=(W=0.000000,X=1.000000,Y=0.000000,Z=0.000000),YPlane=(W=0.000000,X=0.000000,Y=1.000000,Z=0.000000),ZPlane=(W=0.000000,X=0.000000,Y=0.000000,Z=1.000000),WPlane=(W=1.000000,X=0.000000,Y=0.000000,Z=0.000000))" "0.000000,0.000000,0.000000|0.000000,0.000000,0.000000|1.000000,1.000000,1.000000" 1e+02 (Utilities|Array|MakeArray "OZFusion"))))
  ;[1 1 1] Merge meshes in a single SkeletalMesh
  (bind _returnvalue_2 (Class|GlTFRuntimeAsset|LoadSkeletalMeshRecursive _returnvalue "RootNode" 0 (Utilities|Struct|MakeglTFRuntimeSkeletalMeshConfig "ReadWrite" "/OZFusion/Animations/Model/BitmojiSkeleton.BitmojiSkeleton" true 0 false -1 "(CacheMode=ReadWrite,bAddRootBone=False,RootBoneName=\"\",BonesNameMap=(),BonesTransformMap=(),bNormalizeSkeletonScale=False,RootNodeIndex=-1,Sockets=())" "(CacheMode=ReadWrite,UberMaterialsOverrideMap=(),MaterialsOverrideMap=(),TexturesOverrideMap=(),ImagesOverrideMap=(),bDisableVertexColors=False,bGeneratesMipMaps=False,bMergeSectionsByMaterial=False,SpecularFactor=0.000000)" 0 "5.000000,2.000000,1.000000" true)))
  ;[1 1 1] Fix MSkeletalMesh and Capsule
  (bind _output_get (Variables|Default|SetglTFSkeletalMesh _returnvalue_2))
  (bind _output_get_2 (Variables|Default|SetDancerHalfHeight (.z (.boxextent (StaticMesh|GetBounds _output_get)))))
  (Components|Capsule|SetCapsuleHalfHeight (Variables|Collision|GetCapsuleComponent) _output_get_2 true)
  (Transformation|AddLocalOffset (Variables|Character|GetMesh) (Math|Vector|MakeVector 0.0 0.0 (* (Variables|Default|GetDancerHalfHeight) -1.0)) false false)
  ;[1 1 1] Assign the SkeletalMesh
  (Class|SkinnedMeshComponent|SetSkeletalMesh (Variables|Character|GetMesh) (Variables|Default|GetglTFSkeletalMesh) true)
  ;[1 1 1] Only load face if lod0
  (if (Variables|Default|GetHighResolution)
    ;[1 1 1] Load MorphTargets Animation Curves
    (for _array_element_2 (Variables|Default|GetFaces)
      (bind _returnvalue_3 (Class|GlTFRuntimeFunctionLibrary|GlTFLoadAssetfromFilename (Utilities|String|Append "FacialAnimations/" _array_element_2) true (Utilities|Struct|MakeglTFRuntimeConfig "Default" "(XPlane=(W=0.000000,X=1.000000,Y=0.000000,Z=0.000000),YPlane=(W=0.000000,X=0.000000,Y=1.000000,Z=0.000000),ZPlane=(W=0.000000,X=0.000000,Y=0.000000,Z=1.000000),WPlane=(W=1.000000,X=0.000000,Y=0.000000,Z=0.000000))" "0.000000,0.000000,0.000000|0.000000,0.000000,0.000000|1.000000,1.000000,1.000000" 1e+02 (Utilities|Array|MakeArray "OZFusion"))))
      (bind _returnvalue_4 (Class|GlTFRuntimeAsset|LoadSkeletalAnimation _returnvalue_3 (Variables|Default|GetglTFSkeletalMesh) 0 (Utilities|Struct|MakeglTFRuntimeSkeletalAnimationConfig "ReadWrite" -1 false false true true true)))
      (Utilities|Array|Add (Variables|Default|GetFacialAnimations) _returnvalue_4))
    (CallFunction|PlayFacialAnimation)))

(fn ConstructionScript)

(fn GetRandomFacialAnimation
  (bind _facialanimations (Variables|Default|GetFacialAnimations))
  (bind _facialanimations_2 (Variables|Default|GetFacialAnimations))
  (bind _returnvalue (Utilities|Array|Length _facialanimations))
  (bind _returnvalue_2 (- _returnvalue 1))
  (bind _returnvalue_3 (Math|Random|RandomIntegerinRange 0 _returnvalue_2))
  (bind _output (Utilities|Array|Get(acopy) _facialanimations_2 _returnvalue_3))
  (return _output (Variables|/Script/Engine.AnimSequenceBase|GetSequenceLength _output)))