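; Avatar character that loads its glTF model at runtime from content files, at high or low LOD, onto a forced Bitmoji skeleton.
; Initialize starts the async load; the callback fits the capsule, assigns the mesh, initializes the animation blueprint, snaps to its placeholder and acknowledges the spawn to the web controller.
; High-resolution avatars also load morph-target facial animations, played randomly on the Face slot by a re-arming timer.
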(event Custom|PlayFacialAnimation
  ;[1 1 1] Randomly play a facial animation
  (bind (_animation _duration) (CallFunction|GetRandomFacialAnimation))
  (Class|AnimInstance|PlaySlotAnimationasDynamicMontage (Components|SkeletalMesh|GetAnimInstance (Variables|Character|GetMesh)) _animation "Face" 0.25 0.25 1.0 1 -1.0 0.0)
  (Utilities|Time|SetTimerbyEvent (delegate Custom|PlayFacialAnimation) _duration))

(event EventBeginPlay
  ;[1 1 1] Assign placeholder tag
  (Utilities|Array|Add (Variables|Actor|GetTags) (Utilities|String|StringToName "Placeholder")))

(fn ConstructionScript)

(fn Initialize
  (params (Filename :type String) (SceneID :type String) (Placeholder :type Actor%20Object%20Reference) (WebController :type Actor%20Object%20Reference) (InitAnimation :type String))
  (Variables|Default|SetInitialAnimation InitAnimation)
  (bind _asbp_avatar_web_controller (Utilities|Casting|CastToBP_AvatarWebController WebController)
    (:then
      (Variables|Default|SetWebController _asbp_avatar_web_controller))
    (:CastFailed
      _))
  (Variables|Default|SetPlaceholder Placeholder)
  (Variables|Default|SetSceneID SceneID)
  (bind _output_get (Variables|Default|SetFilename Filename))
  (bind _fileexists (CallFunction|CheckifFileExists _output_get))
  (if _fileexists
    ;[1 1 1] load asset
    (bind _returnvalue (Class|GlTFRuntimeFunctionLibrary|GlTFLoadAssetfromFilename (Utilities|String|Append "Models/" _output_get (Utilities|String|SelectString "_lod0.glb" "_lod3.glb" (Variables|Default|GetHighResolution))) true (Utilities|Struct|MakeglTFRuntimeConfig "Default" "(XPlane=(W=0.000000,X=1.000000,Y=0.000000,Z=0.000000),YPlane=(W=0.000000,X=0.000000,Y=1.000000,Z=0.000000),ZPlane=(W=0.000000,X=0.000000,Y=0.000000,Z=1.000000),WPlane=(W=1.000000,X=0.000000,Y=0.000000,Z=0.000000))" "0.000000,0.000000,0.000000|0.000000,0.000000,0.000000|1.000000,1.000000,1.000000" 1e+02 (Utilities|Array|MakeArray "OZFusion"))))
    ;[1 1 1] Merge meshes in a single SkeletalMesh
    (Class|GlTFRuntimeAsset|LoadSkeletalMeshRecursiveAsync _returnvalue "RootNode" 0 (EventDispatchers|CreateEvent :!event WebrequestCallback) (Utilities|Struct|MakeglTFRuntimeSkeletalMeshConfig "ReadWrite" "/OZFusion/Animations/Model/BitmojiSkeleton.BitmojiSkeleton" true 0 false -1 "(CacheMode=ReadWrite,bAddRootBone=False,RootBoneName=\"\",BonesNameMap=(),BonesTransformMap=(),bNormalizeSkeletonScale=False,RootNodeIndex=-1,Sockets=())" "(CacheMode=ReadWrite,UberMaterialsOverrideMap=(),MaterialsOverrideMap=(),TexturesOverrideMap=(),ImagesOverrideMap=(),bDisableVertexColors=False,bGeneratesMipMaps=False,bMergeSectionsByMaterial=False,SpecularFactor=0.000000)" 0 "5.000000,2.000000,1.000000" true true))
    (return true)
    (else
      (return false))))

(fn WebrequestCallback
  (params (SkeletalMesh :type Skeletal%20Mesh%20Object%20Reference))
  (bind _initialanimation (Variables|Default|GetInitialAnimation))
  (bind _placeholder (Variables|Default|GetPlaceholder))
  (bind _initialtransform (Variables|Default|GetInitialTransform))
  (bind _webcontroller (Variables|Default|GetWebController))
  (bind _returnvalue (Transformation|GetActorTransform _placeholder))
  (bind (_location _rotation) (Math|Transform|BreakTransform _initialtransform))
  (bind _returnvalue_2 (Math|Transform|TransformLocation _returnvalue "0, 0,62.000000"))
  (bind _returnvalue_3 (Math|Transform|TransformRotation _returnvalue "0,90.000000, 0"))
  (bind _scale (Math|Transform|BreakTransform _returnvalue))
  (bind _returnvalue_4 (Math|Transform|MakeTransform _returnvalue_2 _returnvalue_3 _scale))
  (if (Utilities|IsValid SkeletalMesh)
    ;[1 1 1] Fix MSkeletalMesh and Capsule
    (bind _output_get (Variables|Default|SetglTFSkeletalMesh SkeletalMesh))
    (bind _output_get_2 (Variables|Default|SetDancerHalfHeight (.z (.boxextent (StaticMesh|GetBounds _output_get)))))
    (Components|Capsule|SetCapsuleHalfHeight (Variables|Collision|GetCapsuleComponent) _output_get_2 true)
    (Transformation|AddLocalOffset (Variables|Character|GetMesh) (Math|Vector|MakeVector 0.0 0.0 (* (Variables|Default|GetDancerHalfHeight) -1.0)) false false)
    ;[1 1 1] Assign the SkeletalMesh
    (Class|SkinnedMeshComponent|SetSkeletalMesh (Variables|Character|GetMesh) (Variables|Default|GetglTFSkeletalMesh) true)
    ;[1 1 1] Assign tag
    (Utilities|Array|Add (Variables|Actor|GetTags) (Utilities|String|StringToName (Variables|Default|GetFilename)))
    ;[1 1 1] Only load face if lod0
    (if (Variables|Default|GetHighResolution)
      ;[1 1 1] Load MorphTargets Animation Curves
      (for _array_element (Variables|Default|GetFaces)
        (bind _returnvalue_5 (Class|GlTFRuntimeFunctionLibrary|GlTFLoadAssetfromFilename (Utilities|String|Append "FacialAnimations/" _array_element) true (Utilities|Struct|MakeglTFRuntimeConfig "Default" "(XPlane=(W=0.000000,X=1.000000,Y=0.000000,Z=0.000000),YPlane=(W=0.000000,X=0.000000,Y=1.000000,Z=0.000000),ZPlane=(W=0.000000,X=0.000000,Y=0.000000,Z=1.000000),WPlane=(W=1.000000,X=0.000000,Y=0.000000,Z=0.000000))" "0.000000,0.000000,0.000000|0.000000,0.000000,0.000000|1.000000,1.000000,1.000000" 1e+02 (Utilities|Array|MakeArray "OZFusion"))))
        (bind _returnvalue_6 (Class|GlTFRuntimeAsset|LoadSkeletalAnimation _returnvalue_5 (Variables|Default|GetglTFSkeletalMesh) 0 (Utilities|Struct|MakeglTFRuntimeSkeletalAnimationConfig "ReadWrite" -1 false false true true true)))
        (Utilities|Array|Add (Variables|Default|GetFacialAnimations) _returnvalue_6))
      (CallFunction|PlayFacialAnimation))
    (bind _asabp_web_avatar_animations (Utilities|Casting|CastToABP_WebAvatarAnimations (Components|SkeletalMesh|GetAnimInstance (Actor|GetComponentbyClass "/Script/Engine.SkeletalMeshComponent")))
      (:then
        (Variables|/OZFusion/Animations/Controllers/ABP_WebAvatarAnimations.ABP_WebAvatarAnimations_C|SetLookAtTarget _asabp_web_avatar_animations (Variables|Default|GetLookAtCameraPosition))
        (Default|Initialize _asabp_web_avatar_animations (Variables|Default|GetSceneID))
        (if (Utilities|Array|IsEmpty _initialanimation)
          _
          (else
            (Default|SetAnimation _asabp_web_avatar_animations _initialanimation)
            (if (Variables|Default|GetRandomAnimSpeed)
              _
              (else
                (Variables|/OZFusion/Animations/Controllers/ABP_WebAvatarAnimations.ABP_WebAvatarAnimations_C|SetplaySpeed _asabp_web_avatar_animations 1.0))))))
      (:CastFailed
        _))
    (if (Utilities|IsValid _placeholder)
      (Transformation|SetActorTransform (Math|Transform|MakeTransform (Math|Transform|TransformLocation _returnvalue_4 _location) (Math|Transform|TransformRotation _returnvalue_4 _rotation) (.Scale (Math|Transform|BreakTransform _returnvalue_4))))))
  (if (Utilities|IsValid _webcontroller)
    (bind _asavatar_placeholder (Utilities|Casting|CastToAvatarPlaceholder (Variables|Default|GetPlaceholder))
      (:then
        (Default|AcknowledgeSpawn _webcontroller _asavatar_placeholder)
        (return))
      (:CastFailed
        (Development|PrintString "failed2cast")))
    (else
      (return))))

(fn GetRandomFacialAnimation
  (bind _facialanimations (Variables|Default|GetFacialAnimations))
  (bind _facialanimations_2 (Variables|Default|GetFacialAnimations))
  (bind _returnvalue (Utilities|Array|Length _facialanimations))
  (bind _returnvalue_2 (- _returnvalue 1))
  (bind _returnvalue_3 (Math|Random|RandomIntegerinRange 0 _returnvalue_2))
  (bind _output (Utilities|Array|Get(acopy) _facialanimations_2 _returnvalue_3))
  (return _output (Variables|/Script/Engine.AnimSequenceBase|GetSequenceLength _output)))

(fn CheckifFileExists
  (params (Filename :type String))
  (bind _highresolution (Variables|Default|GetHighResolution))
  (bind _returnvalue (Utilities|String|SelectString "_lod0.glb" "_lod3.glb" _highresolution))
  (bind _returnvalue_2 (Utilities|String|Append "Models/" Filename _returnvalue))
  (if (or (Class|BlueprintPathsLibrary|FileExists (Utilities|String|Append (Class|KismetSystemLibrary|GetProjectContentDirectory) _returnvalue_2)) (Class|BlueprintPathsLibrary|FileExists (Utilities|String|Append (Utilities|String|Append (Class|KismetSystemLibrary|GetProjectDirectory) "Plugins/OZFusion/Content/") _returnvalue_2)))
    (Variables|Default|SetBooleanHelper true)
    (else
      (bind _output_get (Variables|Default|SetBooleanHelper false))))
  (return _output_get))

(fn SetAnimation
  (params (name :type String))
  (bind _asabp_web_avatar_animations (Utilities|Casting|CastToABP_WebAvatarAnimations (Components|SkeletalMesh|GetAnimInstance (Actor|GetComponentbyClass "/Script/Engine.SkeletalMeshComponent"))))
  (Default|SetAnimation _asabp_web_avatar_animations name))