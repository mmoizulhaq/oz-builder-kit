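; BP_AvatarWebController is a UDP command controller that lets an external app spawn, animate and destroy avatars and pods.
; On BeginPlay it collects AvatarPlaceholders outside pods; the Pods array is not filled here.
; Comma-separated messages route by command name to indexed avatars, PodWithAvatars or a custom event dispatcher, with aliases for standalone avatar animations.
; Replies go back over UDP as Spawn Pod acknowledgements or through EventToApp.
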(event OnReceivedBytes(UDP)
  (params (Bytes :type Array%20of%20Bytes))
  (bind _returnvalue (Class|CUBlueprintLibrary|ToString(Bytes) Bytes))
  (bind (_lefts _rights) (Utilities|String|Split _returnvalue ","))
  (Development|PrintString _returnvalue)
  ;[1 1 1] Parse command
  (switch string _lefts
    (:SpawnAvatar
      (CallFunction|HandleSpawnRequest _rights))
    (:Animation
      (CallFunction|HandleAnimationRequest _rights))
    (:SpawnPod
      (bind (_success _slot) (CallFunction|SpawnPod _rights))
      (CallFunction|Acknowledge _success (Utilities|String|Append _returnvalue "slot=" (Utilities|String|ToString(Integer) _slot))))
    (:SpawnPodMember
      (CallFunction|SpawnPodMember _rights))
    (:DestroyPod
      (CallFunction|DestroyPod _rights))
    (:DestroyPodMember
      (CallFunction|DestroyPodMember _rights))
    (:Custom
      (Default|CallOzEventDispatcher _rights))
    (:DestroyAvatar
      (CallFunction|DestroyAvatar _rights))))

(event EventBeginPlay
  (bind _outactors (Actor|GetAllActorsOfClass "/OZFusion/AvatarPlaceholder.AvatarPlaceholder_C"))
  (bind _array_element (Utilities|Array|ForEachLoopwithBreak _outactors)
    (:LoopBody
      (Utilities|Casting|CastToPodWithAvatars (Actor|GetParentActor _array_element)
        (:CastFailed
          (Utilities|Array|Add (Variables|Default|GetAvatars) _array_element))))))

(fn ConstructionScript)

(fn HandleAnimationRequest
  (params (command :type String))
  (bind (_lefts _rights) (Utilities|String|Split command ","))
  (bind _pods (Variables|Default|Getpods))
  (bind _returnvalue (Math|Conversions|ToInteger(Byte) _lefts))
  (bind (_lefts_2 _rights_2 _returnvalue_2) (Utilities|String|Split _rights ","))
  (Development|PrintString command)
  (if _returnvalue_2
    (if (>= _returnvalue (Utilities|Array|Length _pods))
      (Development|PrintString "Animation pod index out of bounds")
      (else
        (bind _aspod_with_avatars (Utilities|Casting|CastToPodWithAvatars (Utilities|Array|Get(acopy) _pods _returnvalue)))
        (Default|AnimatePodMember _aspod_with_avatars _rights_2 (Math|Conversions|ToInteger(Byte) _lefts_2))))
    (else
      (switch string _rights
        (:Default
          (Variables|Default|Setanimname _rights))
        (:boost-animation-one
          (Variables|Default|Setanimname "selection1"))
        (:boost-animation-two
          (Variables|Default|Setanimname "selection2"))
        (:boost-animation-three
          (Variables|Default|Setanimname "winner"))
        (:boost-animation-four
          (Variables|Default|Setanimname "loser"))
        (:boost-animation-five
          (Variables|Default|Setanimname "floating")))
      (Default|Animate (Utilities|Array|Get(acopy) (Variables|Default|GetAvatars) _returnvalue) (Variables|Default|Getanimname)))))

(fn HandleSpawnRequest
  (params (Filename :type String))
  (bind (_lefts _rights) (Utilities|String|Split Filename ","))
  (bind _avatars (Variables|Default|GetAvatars))
  (bind (_lefts_2 _rights_2 _returnvalue) (Utilities|String|Split _rights ","))
  (bind _returnvalue_2 (Math|Conversions|ToInteger(Byte) _lefts))
  (bind _output (Utilities|Array|Get(acopy) _avatars _returnvalue_2))
  (if (not (Variables|/OZFusion/AvatarPlaceholder.AvatarPlaceholder_C|GetSpawned _output))
    (Default|SpawnAvatar _output (Utilities|String|SelectString _lefts_2 _rights _returnvalue) (Variables|/OZFusion/AvatarPlaceholder.AvatarPlaceholder_C|GetHigh%20resolution _output) (Utilities|String|SelectString _rights_2 "" _returnvalue))))

(fn SpawnPod
  (params (filename :type String))
  (bind (_lefts _rights) (Utilities|String|Split filename ","))
  (bind _pods (Variables|Default|Getpods))
  (bind _returnvalue (Utilities|Array|Length _pods))
  (bind _returnvalue_2 (Math|Conversions|ToInteger(Byte) _lefts))
  (if (== _returnvalue 0)
    (Development|PrintString "Aborting spawn with no pods found")
    (return false _returnvalue_2)
    (elif (>= _returnvalue_2 _returnvalue)
      (Development|PrintString "Pod spawn index out of bounds")
      (return false _returnvalue_2)
      (else
        (bind _aspod_with_avatars (Utilities|Casting|CastToPodWithAvatars (Utilities|Array|Get(acopy) _pods _returnvalue_2)))
        (Default|SpawnPod _aspod_with_avatars _rights)))))

(fn SpawnPodMember
  (params (Filename :type String))
  (bind (_lefts _rights) (Utilities|String|Split Filename ","))
  (bind _pods (Variables|Default|Getpods))
  (bind _returnvalue (Math|Conversions|ToInteger(Byte) _lefts))
  (bind (_lefts_2 _rights_2) (Utilities|String|Split _rights ","))
  (if (>= _returnvalue (Utilities|Array|Length _pods))
    (Development|PrintString "Out of bounds")
    (else
      (bind _aspod_with_avatars (Utilities|Casting|CastToPodWithAvatars (Utilities|Array|Get(acopy) _pods _returnvalue)))
      (Default|SpawnPodMember _aspod_with_avatars _rights_2 (Math|Conversions|ToInteger(Byte) _lefts_2)))))

(fn Acknowledge
  (params (Success :type Boolean) (Command :type String))
  (Class|UDPComponent|EmitBytes (Variables|Default|GetUDP) (Class|CUBlueprintLibrary|ToBytes(String) (Utilities|String|Append "success=" (Utilities|String|ToString(Boolean) Success) "command=" Command))))

(fn DestroyPod
  (params (Slot :type String))
  (bind _returnvalue (Math|Conversions|ToInteger(Byte) Slot))
  (bind _pods (Variables|Default|Getpods))
  (if (>= _returnvalue (Utilities|Array|Length _pods))
    (Development|PrintString "Destroying pod index out of bounds")
    (return)
    (else
      (bind _aspod_with_avatars (Utilities|Casting|CastToPodWithAvatars (Utilities|Array|Get(acopy) _pods _returnvalue)))
      (Default|DestroyPod _aspod_with_avatars))))

(fn DestroyPodMember
  (params (Slot :type String))
  (bind (_lefts _rights) (Utilities|String|Split Slot ","))
  (bind _pods (Variables|Default|Getpods))
  (bind _returnvalue (Math|Conversions|ToInteger(Byte) _lefts))
  (if (>= _returnvalue (Utilities|Array|Length _pods))
    (Development|PrintString "Destroying pod index out of bounds")
    (return)
    (else
      (bind _aspod_with_avatars (Utilities|Casting|CastToPodWithAvatars (Utilities|Array|Get(acopy) _pods _returnvalue)))
      (Default|DestroyPodMember _aspod_with_avatars (Math|Conversions|ToInteger(Byte) _rights)))))

(fn EventtoApp
  (params (Event :type String))
  (Class|UDPComponent|EmitBytes (Variables|Default|GetUDP) (Class|CUBlueprintLibrary|ToBytes(String) Event)))

(fn DestroyAvatar
  (params (Location :type String))
  (Default|DestroyAvatar (Utilities|Array|Get(acopy) (Variables|Default|GetAvatars) (Math|Conversions|ToInteger(Byte) Location))))